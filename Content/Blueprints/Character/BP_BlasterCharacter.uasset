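; Blueprint for the Blaster character that drives its overhead widget, a debug and identity label.
; On BeginPlay it casts the widget component's object to WBP_OverheadWidget and shows the character's net role.
; Every Tick it repeats the cast and refreshes the player name.
; Disconnected debug sphere nodes remain from testing the range of the shell sound cue.
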(event EventBeginPlay
  (bind _aswbp_overhead_widget (Utilities|Casting|CastToWBP_OverheadWidget (UserInterface|GetUserWidgetObject (Variables|Default|GetOverheadWidget))))
  (Class|OverheadWidget|ShowPlayerNetRole _aswbp_overhead_widget self))

(event Collision|EventActorBeginOverlap
  (params (OtherActor :type Actor%20Object%20Reference)))

(event EventTick
  (params (DeltaSeconds :type Float%20%28single-precision%29))
  (bind _aswbp_overhead_widget (Utilities|Casting|CastToWBP_OverheadWidget (UserInterface|GetUserWidgetObject (Variables|Default|GetOverheadWidget))))
  (Class|OverheadWidget|ShowPlayerName _aswbp_overhead_widget self))

(fn ConstructionScript)